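; Falling platform that drops shortly after the player character steps on it, then returns to its starting position to be used again.
; A box overlap with the custom third-person character triggers a warning delay, then the cube simulates physics and falls for a few seconds.
; A timeline lerps it back to its saved transform and re-arms it.
; Material swaps show each state: steady, activated, falling and resetting.
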(event `self.ReceiveBeginPlay`
  (set `self.StartingTransform` (`SceneComponent.K2_GetComponentToWorld` (`self.Cube`))) ; Saving starting location and rotation of the platform
  (`PrimitiveComponent.SetMaterial` (`self.Cube`) 0 "/Game/Materials/PlatformSteady.PlatformSteady"))

(event `self.Box.OnComponentBeginOverlap`
  (params (OverlappedComponent :type "PrimitiveComponent Object Reference") (OtherActor :type "Actor Object Reference") (OtherComp :type "PrimitiveComponent Object Reference") (OtherBodyIndex :type Integer) (bFromSweep :type Boolean) (SweepResult :type "HitResult Structure (by ref)"))
  (cast `/Game/Blueprints/BP_ThirdPersonCharacter-Custom` OtherActor)
  (`self.Activate`))

(event `Activate`
  ;[1 0.9807 0.1389] PlatformActivates
  (if (`self.Ready`)
    (`KismetSystemLibrary.PrintString` "The Platform is about to drop!")
    (set `self.Ready` false)
    (`PrimitiveComponent.SetMaterial` (`self.Cube`) 0 "/Game/Materials/PlatformActivated.PlatformActivated")
    (`KismetSystemLibrary.Delay` 1.0)
    (`self.Drop`)))

(event `Drop`
  ;[1 0.1018 0.1237] PlatformDrops for 3 Seconds
  (`KismetSystemLibrary.PrintString` "Dropping")
  (`PrimitiveComponent.SetSimulatePhysics` (`self.Cube`) true)
  (`PrimitiveComponent.SetMaterial` (`self.Cube`) 0 "/Game/Materials/PlatformFalling.PlatformFalling")
  (`KismetSystemLibrary.Delay` 3.0)
  (`self.Reset`))

(event `Reset`
  ;[0.1955 1 0.1363] Platform Resets for 3 Seconds
  (`KismetSystemLibrary.PrintString` "Resetting")
  (set `self.EndTransform` (`SceneComponent.K2_GetComponentToWorld` (`self.Cube`)))
  (`PrimitiveComponent.SetMaterial` (`self.Cube`) 0 "/Game/Materials/PlatformResetting.PlatformResetting")
  (`PrimitiveComponent.SetSimulatePhysics` (`self.Cube`) false)
  (bind (_direction _reset_float) (`Timeline|GoBacktoStart` :!via `PlayFromStart`)
    (:`Update`
      (bind (_returnvalue_location _returnvalue_rotation) (`KismetMathLibrary.BreakTransform` (`KismetMathLibrary.TLerp` (`self.EndTransform`) (`self.StartingTransform`) _reset_float)))
      (`SceneComponent.K2_SetWorldLocationAndRotation` (`self.Cube`) _returnvalue_location _returnvalue_rotation false false))
    (:`Finished`
      (set `self.Ready` true)
      (`PrimitiveComponent.SetMaterial` (`self.Cube`) 0 "/Game/Materials/PlatformSteady.PlatformSteady"))))

(fn `UserConstructionScript`)