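; Tutorial Blueprint demonstrating loops and arrays through printed strings and a key color effect.
; Input triggers a counted while loop within one frame, a numbered ForEach name list and an array length printout.
; BeginPlay gathers BP_Key actors, then ChangeKeyColor re-calls itself after a delay, tinting one key per step via dynamic materials and reshuffling both arrays.
; The simple, recursive and Tick examples are left unconnected from their events.
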(event `RecursiveLoop`
  ;[0.548 0.44 1] Recursive Loop
)

(event `FirstArrayTest`
  (`KismetSystemLibrary.PrintString` (`KismetStringLibrary.Concat_StrStr` "Our array of names is " (`KismetStringLibrary.Conv_IntToString` (`KismetArrayLibrary.Array_Length` (`|MakeArray` "Luke" "Han" "Leia" "Chewie" "Artoo" "Threepio"))) " names long")))

(event `Key|Five`
  (params (Key :type "Key Structure"))
  (:`Pressed`
    (`self.ListofNames`)))

(event `Key|Six`
  (params (Key :type "Key Structure"))
  (:`Pressed`
    (`self.FirstArrayTest`)))

(event `ListofNames`
  (for (_array_element _array_index) (`|MakeArray` "Luke" "Han" "Leia" "Chewie" "Artoo" "Threepio")
    (`KismetSystemLibrary.PrintString` (`KismetStringLibrary.Concat_StrStr` (`KismetStringLibrary.Conv_IntToString` (+ _array_index 1)) ". " _array_element))))

(event `InputAction|Start While Loop`
  (params (Key :type "Key Structure"))
  (bind _whileloopcounter (`self.WhileLoopCounter`))
  (:`Pressed`
    (`KismetSystemLibrary.PrintString` "Starting While Opp")
    (while (< (`self.WhileLoopCounter`) 25)
      ;[0.176 0.5666 1] LoopBody
      (`/Engine/EditorBlueprintResources/StandardMacros.IncrementInt` _whileloopcounter
        (:`  `
          (`KismetSystemLibrary.PrintString` (`KismetStringLibrary.Concat_StrStr` "This string has run" (`KismetStringLibrary.Conv_IntToString` _whileloopcounter) "times") true true (`KismetMathLibrary.MakeColor` (`KismetMathLibrary.RandomFloat`) (`KismetMathLibrary.RandomFloat`) (`KismetMathLibrary.RandomFloat`))))))
    (`KismetSystemLibrary.PrintString` "The While Loop is done")
    (set `self.WhileLoopCounter` 0)))

(event `self.ReceiveBeginPlay`
  (`KismetSystemLibrary.PrintString` "Loops and Lists is starting")
  (`|ExecutionSequence`
    (:`then_0`
      ;[1 0.3499 0.3001] Setup for Loops
      (`self.Simple Game Loop`)
      (`self.EnableInput` (`GameplayStatics.GetPlayerController` 0))
      (`self.RecursiveLoop`))
    (:`then_1`
      ;[0.2721 1 0.4372] Setup for Lists
      (bind _outactors (`GameplayStatics.GetAllActorsOfClass` "/Game/Blueprints/BP_Key.BP_Key_C"))
      (set `self.Keys` _outactors)
      (`self.Change Key Color`))))

(event `Change Key Color`
  (bind _keys (`self.Keys`))
  (bind _output (`|GetArrayItem` _keys (`self.Color Key Index`)))
  ;[1 1 1 0.487 73] Key Color Randomizer
  (if (or (>= (`self.Color Key Index`) (`KismetArrayLibrary.Array_Length` (`self.Colors`))) (>= (`self.Color Key Index`) (`KismetArrayLibrary.Array_Length` (`self.Keys`))))
    ;;[0.3291 0.3289 1] Shuffle and Reset
    (`KismetArrayLibrary.Array_Shuffle` (`self.Colors`)) ; Shuffle order of colors
    (`KismetArrayLibrary.Array_Shuffle` _keys) ; Shuffle Order of keys
    (set `self.Color Key Index` 0))
  (`/Engine/EditorBlueprintResources/StandardMacros.IsValid` _output ; Does the Key still exist
    (:`Is Valid`
      ;;[0.5276 1 0.1707] Setting the Color
      (bind _returnvalue (`PrimitiveComponent.CreateDynamicMaterialInstance` (`/Game/Blueprints/BP_Key.Cylinder` _output) 0 "/Game/Materials/M_Base.M_Base" "None"))
      (`MaterialInstanceDynamic.SetVectorParameterValue` _returnvalue "Base Color" (`KismetMathLibrary.Conv_ColorToLinearColor` (`|GetArrayItem` (`self.Colors`) (`self.Color Key Index`)))))
    (:`Is Not Valid`
      (bind _outactors (`GameplayStatics.GetAllActorsOfClass` "/Game/Blueprints/BP_Key.BP_Key_C"))
      (set `self.Keys` _outactors)))
  (`/Engine/EditorBlueprintResources/StandardMacros.IncrementInt` (`self.Color Key Index`)
    (:`  `
      (`KismetSystemLibrary.Delay` 0.5)
      (`self.Change Key Color`))))

(event `Simple Game Loop`
  ;[1 1 1 1 37] Simple Loop
)

(event `self.ReceiveTick`
  (params (DeltaSeconds :type "Float (single-precision)"))
  ;[1 1 1 1 44] Game Tick
)

(fn `UserConstructionScript`)