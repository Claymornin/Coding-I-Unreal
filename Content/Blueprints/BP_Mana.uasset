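; BP_Mana is a holdable mana can pickup that is consumed on use, though its mana gain is only a debug print.
; Overlapping its trigger asks the custom third-person character to pick it up, and the Pickup event attaches it to the hand_r socket.
; Drop detaches it and enables physics and collision on the can.
; Primary action prints the gain, clears the character's HeldItem and destroys the actor, while secondary action only prints a placeholder.
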(event `self.PickupTrigger.OnComponentBeginOverlap`
  (params (OverlappedComponent :type "PrimitiveComponent Object Reference") (OtherActor :type "Actor Object Reference") (OtherComp :type "PrimitiveComponent Object Reference") (OtherBodyIndex :type Integer) (bFromSweep :type Boolean) (SweepResult :type "HitResult Structure (by ref)"))
  ;[1 1 1] Pick Up (Item End)
  (bind _asbp_third_person_character__custom (cast `/Game/Blueprints/BP_ThirdPersonCharacter-Custom` OtherActor))
  (`/Game/Blueprints/BP_ThirdPersonCharacter-Custom.Try to Pick Up` _asbp_third_person_character__custom self))

(event `self.Pickup`
  (params (ParentMesh :type "SkeletalMeshComponent Object Reference"))
  ;[0.3115 0.3115 0.3115] Successful Pick Up
  (`SceneComponent.K2_AttachToComponent` (`self.DefaultSceneRoot`) ParentMesh "hand_r" "SnapToTarget" "KeepRelative" "KeepRelative" true))

(event `self.Drop`
  (`SceneComponent.K2_DetachFromComponent` (`self.DefaultSceneRoot`) "KeepRelative" "KeepRelative" "KeepRelative" true)
  (`PrimitiveComponent.SetSimulatePhysics` (`self.Can`) true)
  (`PrimitiveComponent.SetCollisionEnabled` (`self.Can`) "QueryAndPhysics"))

(event `self.PrimaryAction`
  (params (ref_ThirdPersonCharCust :type "/Game/Blueprints/BP_ThirdPersonCharacter-Custom Object Reference"))
  (`KismetSystemLibrary.PrintString` "+10 Mana")
  (set `/Game/Blueprints/BP_ThirdPersonCharacter-Custom.HeldItem` null ref_ThirdPersonCharCust)
  (`self.K2_DestroyActor`))

(event `/Game/Blueprints/BPI_Item.SecondaryAction`
  (`KismetSystemLibrary.PrintString` "Here's your secondary action!" true true (struct :`R` 1.0 :`G` 0.094673 :`B` 0.138459 :`A` 1.0)))

(fn `UserConstructionScript`)