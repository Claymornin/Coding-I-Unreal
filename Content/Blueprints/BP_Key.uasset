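; BP_Key is a collectible key pickup that the player gathers by walking into its box collision.
; On overlap it casts the other actor to BP_ThirdPersonCharacter-Custom, increments that character's KeyCount, then destroys itself.
; Debug screen prints report its spawn, each pickup with the new key total, and failed casts.
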(event `self.ReceiveBeginPlay`
  (`KismetSystemLibrary.PrintString` "This Key Exists" true true (struct :`R` 1.0 :`G` 0.094565 :`B` 0.890759 :`A` 1.0) 5.0))

(event `self.Box Collision.OnComponentBeginOverlap`
  (params (OverlappedComponent :type "PrimitiveComponent Object Reference") (OtherActor :type "Actor Object Reference") (OtherComp :type "PrimitiveComponent Object Reference") (OtherBodyIndex :type Integer) (bFromSweep :type Boolean) (SweepResult :type "HitResult Structure (by ref)"))
  (bind _asbp_third_person_character__custom (cast `/Game/Blueprints/BP_ThirdPersonCharacter-Custom` OtherActor)
    (:`then`
      (`KismetSystemLibrary.PrintString` "A Player Ran into Me!" true true (struct :`G` 0.66 :`B` 1.0 :`A` 1.0) 5.0)
      (bind _key_count (`/Game/Blueprints/BP_ThirdPersonCharacter-Custom.key Count` _asbp_third_person_character__custom))
      (set `/Game/Blueprints/BP_ThirdPersonCharacter-Custom.key Count` (+ _key_count 1) _asbp_third_person_character__custom) ; Set Key Count
      (`KismetSystemLibrary.PrintString` (`KismetStringLibrary.Concat_StrStr` "The Player has " (`KismetStringLibrary.Conv_IntToString` _key_count) " Keys"))
      (`self.K2_DestroyActor`) ; Destroy this Key
    )
    (:`CastFailed`
      (`KismetSystemLibrary.PrintString` "Key Player Cast Failed" true true (struct :`R` 1.0 :`G` 0.044733 :`B` 0.088518 :`A` 1.0) 5.0))))

(fn `UserConstructionScript`)